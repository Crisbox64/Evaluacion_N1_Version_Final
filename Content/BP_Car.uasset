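; BP_Car is a car Blueprint that endlessly cycles the material on two of its components, Cube and Cube1.
; BeginPlay runs a looping chain of Delays, applying four materials in turn at two-second intervals to the first material slot of both components.
; The loop wires back to its first Delay, so it needs no Tick or timer, and the construction script is empty.
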(event `self.ReceiveBeginPlay`
  (`KismetSystemLibrary.Delay` 2.0 :!label _label)
  (`PrimitiveComponent.SetMaterial` (`self.Cube`) 0 "/Game/Materials/Material19.Material19")
  (`PrimitiveComponent.SetMaterial` (`self.Cube1`) 0 "/Game/Materials/Material19.Material19")
  (`KismetSystemLibrary.Delay` 2.0)
  (`PrimitiveComponent.SetMaterial` (`self.Cube`) 0 "/Game/Materials/Material20.Material20")
  (`PrimitiveComponent.SetMaterial` (`self.Cube1`) 0 "/Game/Materials/Material20.Material20")
  (`KismetSystemLibrary.Delay` 2.0)
  (`PrimitiveComponent.SetMaterial` (`self.Cube`) 0 "/Game/Materials/Material9.Material9")
  (`PrimitiveComponent.SetMaterial` (`self.Cube1`) 0 "/Game/Materials/Material9.Material9")
  (`KismetSystemLibrary.Delay` 2.0)
  (`PrimitiveComponent.SetMaterial` (`self.Cube`) 0 "/Game/Materials/Material17.Material17")
  (`PrimitiveComponent.SetMaterial` (`self.Cube1`) 0 "/Game/Materials/Material17.Material17")
  (goto _label))

(fn `UserConstructionScript`)